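; Base Blueprint for Stone Age plants, which loads its sub-resource data when play begins.
; BeginPlay caches the ResourceGameInstance, then uses SubResourceName to fetch and store the matching SubResourceStruct from it.
; The construction script only calls the parent class version.
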(event `self.ReceiveBeginPlay`
  (`self.CreateReferences`)
  (`self.SetInfo`))

(fn `UserConstructionScript`
  (`parent.UserConstructionScript`))