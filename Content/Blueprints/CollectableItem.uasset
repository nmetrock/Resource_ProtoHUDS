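; CollectableItem is a harvestable resource actor that opens a gather menu when clicked within range.
; Delayed setup resolves or randomizes its resource names through the game instance, registers it and rolls health stats.
; Overlap or hover shows a name widget, custom-depth highlight and lerped scale pop; leaving range cancels gathering.
; Tick timers regenerate or decay stack resources, while gathering credits the game instance and moves dependent drops to ground resources.
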(event OnBeginCursorOver(ClickBox)
  (params (TouchedComponent :type Primitive%20Component%20Object%20Reference))
  ;[1 1 1] OverLap and MouseOver Events
  (bind _output_get (Variables|Interaction|SetMouseOver true))
  (if (Class|KismetMathLibrary|XORBoolean (stale OnComponentBeginOverlap(OverlapBox) _output_get) _output_get)
    (|PopupNameWidget
      (:then
        (|VisualEffects :!label _label))
      (:then2
        (goto _label execute2)))))

(event OnComponentBeginOverlap(OverlapBox)
  (params (OverlappedComponent :type Primitive%20Component%20Object%20Reference) (OtherActor :type Actor%20Object%20Reference) (OtherComp :type Primitive%20Component%20Object%20Reference) (OtherBodyIndex :type Integer) (bFromSweep :type Boolean) (SweepResult :type Hit%20Result%20Structure%20%28by%20ref%29))
  ;[1 1 1] OverLap and MouseOver Events
  (bind _output_get (Variables|Interaction|SetOverlapped true))
  (|CheckRangeAndCancelGather
    (:then
      (if (Class|KismetMathLibrary|XORBoolean _output_get (stale OnBeginCursorOver(ClickBox) _output_get))
        (|PopupNameWidget :!label _label
          (:then
            (|VisualEffects :!label _label_2))
          (:then2
            (goto _label_2 execute2)))))
    (:then2
      (if (and (not (stale OnComponentEndOverlap(OverlapBox) _output_get)) (not (stale OnEndCursorOver(ClickBox) _output_get)))
        (goto _label execute2)))))

(event OnComponentEndOverlap(OverlapBox)
  (params (OverlappedComponent :type Primitive%20Component%20Object%20Reference) (OtherActor :type Actor%20Object%20Reference) (OtherComp :type Primitive%20Component%20Object%20Reference) (OtherBodyIndex :type Integer))
  ;[1 1 1] OverLap and MouseOver Events
  (bind _output_get (Variables|Interaction|SetOverlapped false))
  (|CheckRangeAndCancelGather) ; enters at execute2
)

(event OnEndCursorOver(ClickBox)
  (params (TouchedComponent :type Primitive%20Component%20Object%20Reference))
  ;[1 1 1] OverLap and MouseOver Events
  (bind _output_get (Variables|Interaction|SetMouseOver false))
  (if (and (not (stale OnComponentEndOverlap(OverlapBox) _output_get)) (not _output_get))
    (|PopupNameWidget) ; enters at execute2
  ))

(event OnClicked(ClickBox)
  (params (TouchedComponent :type Primitive%20Component%20Object%20Reference) (ButtonPressed :type Key%20Structure :default "None"))
  (bind _gameinstance_ref (Variables|References|GetGameInstance_REF))
  ;[1 1 1] Harvest Menu on Clicked
  (if (Default|GetItemWithinRange (Variables|References|GetGameInstance_REF) "NewEnumerator1" (Variables|ItemInfo|GetSubResourceName))
    (if (Variables|Gathering|GetBeingGathered)
      (Default|AddInstantMessage (Variables|References|GetGameInstance_REF) "Already gathering this resource!")
      (else
        (Default|SetItemClicked _gameinstance_ref true)
        (Default|ClearMenus _gameinstance_ref)
        (Utilities|HarvestMenu)))
    (else
      (Default|AddInstantMessage (Variables|References|GetGameInstance_REF) "Too far away!"))))

(event EventTick
  (params (DeltaSeconds :type Float%20%28single-precision%29))
  ;[1 1 1] Event Tick
  (|Throbber DeltaSeconds)
  (EventTick|RegenorDecay DeltaSeconds))

(event EventBeginPlay
  ;[1 1 1] Begin Play / Set Info
  (Utilities|SetReferences)
  (Utilities|SetVariables)
  (Utilities|Time|SetTimerbyFunctionName 0 "SetInfo" 0.2))

(fn ConstructionScript)

(fn SetInfo
  (|Basicsetup)
  (|SetInfo)
  ;[1 1 1] Add item to list
  (Default|AddAvailableSubResource (Variables|References|GetGameInstance_REF) self))

(fn CheckandSetNames
  (if (Utilities|Name|Equal(Name) (Variables|ItemInfo|GetSourceName) "None")
    (if (Utilities|Name|Equal(Name) (Variables|ItemInfo|GetTopResourceName) "None")
      (if (Utilities|Name|Equal(Name) (Variables|ItemInfo|GetSubResourceName) "None")
        (Development|PrintString (Variables|References|GetErrorNoName))
        (Actor|DestroyActor)
        (else
          (|SetfromSubResource)
          (if (LocalVariables|GetIsValid) :!label _label
            (Variables|ItemInfo|SetResourceNames (Utilities|Struct|BreakSubResourceNames_STRUCT (.SubResourceSTRUCT (Default|GetSubResourceNames (Variables|References|GetGameInstance_REF) (Variables|ItemInfo|GetSubResourceName)))))
            (return)
            (else
              (Development|PrintString (Utilities|String|ToString(Text) (Utilities|Text|FormatText (Utilities|GetDisplayName self) "->CollectableItem ERROR!   Actor destroyed: {self}")))
              (Actor|DestroyActor)))))
      (else
        (|SetRandomfromTopResource)
        (goto _label)))
    (else
      (|SetRandomFromSource)
      (goto _label))))

(fn RegenorDecay
  (params (DeltaSeconds :type Float%20%28single-precision%29))
  (bind _resourcestruct_local (LocalVariables|GetResourceStruct_LOCAL))
  (bind (_currenthealth _maxhealth) (Utilities|Struct|BreakResource_STRUCT _resourcestruct_local))
  (LocalVariables|SetDelta_LOCAL DeltaSeconds)
  (for _array_element (Variables|ItemInfo|GetResourceNames)
    (LocalVariables|SetName_LOCAL _array_element)
    (|SetLocalVariables)
    (|IsHealthAtMax
      (:False
        (|SaveandCheckTimer
          (:Timer%20Full
            (if (< _currenthealth _maxhealth)
              (Gathering|RemovefromStack (LocalVariables|GetName_LOCAL))
              (else
                (|AddorSubtractHealth)
                (bind _structout (Utilities|Struct|SetmembersinResource_STRUCT (LocalVariables|GetResourceStruct_LOCAL) (LocalVariables|GetUpdatedHealth_LOCAL)))
                (Utilities|Map|Add (Variables|ItemInfo|GetStackResources) (LocalVariables|GetName_LOCAL) _structout))))))))
  (return))

(fn SetBeingGathered
  (params (BeingGathered :type Boolean))
  (bind _output_get (Variables|Gathering|SetBeingGathered BeingGathered))
  (return _output_get))

(fn GatherResource
  (params (ResourceName :type Name%20%28by%20ref%29))
  (LocalVariables|SetName_LOCAL ResourceName)
  (LocalVariables|SetStruct_LOCAL (.Value (Utilities|Map|Find (Variables|ItemInfo|GetStackResources) (LocalVariables|GetName_LOCAL))))
  (LocalVariables|SetPercentGathered_LOCAL (/ (Math|Conversions|ToFloat(Integer) (Default|GetGatherQuantity (Variables|References|GetGameInstance_REF) (LocalVariables|GetName_LOCAL))) (Math|Conversions|ToFloat(Integer) (.MaxHealth (Utilities|Struct|BreakResource_STRUCT (LocalVariables|GetStruct_LOCAL))))))
  (LocalVariables|SetGatherQuantity_LOCAL (Math|Integer|Clamp(Integer) (Default|GetGatherQuantity (Variables|References|GetGameInstance_REF) (LocalVariables|GetName_LOCAL)) 0 (.CurrentHealth (Utilities|Struct|BreakResource_STRUCT (LocalVariables|GetStruct_LOCAL)))))
  (bind _output_get (LocalVariables|SetNewHealth_LOCAL (- (.CurrentHealth (Utilities|Struct|BreakResource_STRUCT (LocalVariables|GetStruct_LOCAL))) (Math|Integer|Clamp(Integer) (Default|GetGatherQuantity (Variables|References|GetGameInstance_REF) (LocalVariables|GetName_LOCAL)) 0 (.CurrentHealth (Utilities|Struct|BreakResource_STRUCT (LocalVariables|GetStruct_LOCAL)))))))
  (bind _structout (Utilities|Struct|SetmembersinResource_STRUCT (LocalVariables|GetStruct_LOCAL) _output_get))
  (Utilities|Map|Add (Variables|ItemInfo|GetStackResources) (LocalVariables|GetName_LOCAL) _structout)
  (Default|IncrementResource (Variables|References|GetGameInstance_REF) (LocalVariables|GetName_LOCAL) (LocalVariables|GetGatherQuantity_LOCAL))
  (if (== (LocalVariables|GetNewHealth_LOCAL) 0)
    (Gathering|RemovefromStack (LocalVariables|GetName_LOCAL))
    (return (LocalVariables|GetGatherQuantity_LOCAL))
    (else
      (Gathering|PercentfromStack (LocalVariables|GetName_LOCAL) (LocalVariables|GetPercentGathered_LOCAL))
      (return (LocalVariables|GetGatherQuantity_LOCAL)))))

(fn GetHealthStatus
  (params (ResourceName :type Name%20%28by%20ref%29))
  (bind _stackresources (Variables|ItemInfo|GetStackResources))
  (bind _groundresources (Variables|ItemInfo|GetGroundResources))
  (bind (_value _returnvalue) (Utilities|Map|Find _stackresources ResourceName))
  (bind _value_2 (Utilities|Map|Find _groundresources ResourceName))
  (bind (_currenthealth _maxhealth _regenremaining _regenrate _regenstatus) (Utilities|Struct|BreakResource_STRUCT _value_2))
  (bind (_currenthealth_2 _maxhealth_2 _regenremaining_2 _regenrate_2 _regenstatus_2) (Utilities|Struct|BreakResource_STRUCT _value))
  (if _returnvalue
    (return _currenthealth_2 _maxhealth_2 _regenremaining_2 _regenrate_2 _regenstatus_2)
    (else
      (return _currenthealth _maxhealth _regenremaining _regenrate _regenstatus))))

(fn GetResourceNames
  (bind _keys (Utilities|Map|Keys (Variables|ItemInfo|GetStackResources)))
  (bind _keys_2 (Utilities|Map|Keys (Variables|ItemInfo|GetGroundResources)))
  (return _keys _keys_2))

(fn GetSourceName
  (return (Variables|ItemInfo|GetSourceName)))

(fn GetResourceCount
  (params (ResourceName :type Name%20%28by%20ref%29))
  (bind _stackresources (Variables|ItemInfo|GetStackResources))
  (bind (_value _returnvalue) (Utilities|Map|Find _stackresources ResourceName))
  (if _returnvalue
    (LocalVariables|SetReturnValue_LOCAL (Utilities|Struct|BreakResource_STRUCT _value))
    (return (LocalVariables|GetReturnValue_LOCAL))
    (else
      (LocalVariables|SetReturnValue_LOCAL (Utilities|Struct|BreakResource_STRUCT (.Value (Utilities|Map|Find (Variables|ItemInfo|GetGroundResources) ResourceName))))
      (return (LocalVariables|GetReturnValue_LOCAL)))))

(fn PercentfromStack
  (params (ResourceName :type Name%20%28by%20ref%29) (PercentGathered :type Float%20%28single-precision%29))
  (LocalVariables|SetPercent_LOCAL PercentGathered)
  (for _array_element (.Drops (Utilities|Struct|BreakGathering_STRUCT (.ResourceGathering%20STRUCT (Default|GetGatheringInfo (Variables|References|GetGameInstance_REF) ResourceName))))
    (bind _structout (Utilities|Struct|SetmembersinResource_STRUCT (.Value (Utilities|Map|Find (Variables|ItemInfo|GetStackResources) _array_element)) (Math|Float|Truncate (* (.MaxHealth (Utilities|Struct|BreakResource_STRUCT (.Value (Utilities|Map|Find (Variables|ItemInfo|GetStackResources) _array_element)))) (LocalVariables|GetPercent_LOCAL))) "NewEnumerator1"))
    (Utilities|Map|Add (Variables|ItemInfo|GetGroundResources) _array_element _structout)
    (bind _structout_2 (Utilities|Struct|SetmembersinResource_STRUCT (.Value (Utilities|Map|Find (Variables|ItemInfo|GetStackResources) _array_element)) (- (.CurrentHealth (Utilities|Struct|BreakResource_STRUCT (.Value (Utilities|Map|Find (Variables|ItemInfo|GetStackResources) _array_element)))) (Math|Float|Truncate (* (.MaxHealth (Utilities|Struct|BreakResource_STRUCT (.Value (Utilities|Map|Find (Variables|ItemInfo|GetStackResources) _array_element)))) (LocalVariables|GetPercent_LOCAL))))))
    (Utilities|Map|Add (Variables|ItemInfo|GetStackResources) _array_element _structout_2)))

(fn RemovefromStack
  (params (ResourceName :type Name%20%28by%20ref%29))
  (Utilities|Map|Remove (Variables|ItemInfo|GetStackResources) ResourceName)
  (for _array_element (.Drops (Utilities|Struct|BreakGathering_STRUCT (.ResourceGathering%20STRUCT (Default|GetGatheringInfo (Variables|References|GetGameInstance_REF) ResourceName))))
    (bind _structout (Utilities|Struct|SetmembersinResource_STRUCT (.Value (Utilities|Map|Find (Variables|ItemInfo|GetStackResources) _array_element)) "NewEnumerator1"))
    (Utilities|Map|Add (Variables|ItemInfo|GetGroundResources) _array_element _structout)
    (Utilities|Map|Remove (Variables|ItemInfo|GetStackResources) _array_element)))