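; Master item actor, apparently a base for items, that loads its source data by name at BeginPlay.
; It caches a reference to ResourceGameInstance, then asks it for the struct matching SourceName and stores the result.
; An unknown name prints an error and destroys the actor, while a name of "None" skips the lookup and counts as valid.
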(event `self.ReceiveBeginPlay`
  (`self.CreateReferences`)
  (`self.SetSourceStruct` (`self.SourceName`)))

(fn `SetSourceStruct`
  (params (SourceName :type Name))
  (returns (SourceStruct :type "/Game/Struct/Source_STRUCT Structure") (IsValid :type Boolean))
  (bind (_source_struct _isvalid) (`/Game/GameBP/ResourceGameInstance.GetSourceStruct` (`self.GameInstance_REF`) SourceName))
  (if (== SourceName "None")
    (return (struct) true)
    (elif _isvalid
      (bind _output_get (set `self.SourceStruct` _source_struct))
      (return _output_get true)
      (else
        (`KismetSystemLibrary.PrintString` (`KismetTextLibrary.Conv_TextToString` (`|FormatText` "->ERROR, NAME NOT FOUND!   Source: {S}" (`self.SourceName`))))
        (`self.K2_DestroyActor`)
        (return (struct) false)))))

(fn `UserConstructionScript`)